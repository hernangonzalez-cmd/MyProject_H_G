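; BP_Player is the player character, handling Enhanced Input movement, looking, jumping, running and melee attacks.
; It adds the input mapping context on BeginPlay, moves relative to control yaw, and switches walk speed for running.
; Attacks use an AttackIndex to select punch, elbow or kick montages, gated by Canattack and reset on completion.
; HitDetection sphere-traces WorldStatic objects at the matching limb socket with debug drawing, leaving results unused.
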(event `self.ReceiveBeginPlay`
  (bind _asplayer_controller (cast `PlayerController` (`self.GetController`)))
  (bind _returnvalue (pcsubsystem `EnhancedInputLocalPlayerSubsystem` _asplayer_controller))
  (`/Engine/EditorBlueprintResources/StandardMacros.IsValid` _returnvalue
    (:`Is Valid`
      (`EnhancedInputSubsystemInterface.AddMappingContext` _returnvalue "/Game/Integers/IMC_Player.IMC_Player" 0 (struct)))))

(event `EnhancedInput|/Game/Integers/IA_Jump`
  (params (ActionValue :type Boolean) (ElapsedSeconds :type "Float (double-precision)") (TriggeredSeconds :type "Float (double-precision)") (InputAction :type "InputAction Object Reference" :default "/Game/Integers/IA_Jump.IA_Jump"))
  (:`Triggered`
    (`self.Jump`)))

(event `EnhancedInput|/Game/Integers/IA_Look`
  (params (ActionValue :type "Vector2D Structure") (ElapsedSeconds :type "Float (double-precision)") (TriggeredSeconds :type "Float (double-precision)") (InputAction :type "InputAction Object Reference" :default "/Game/Integers/IA_Look.IA_Look"))
  (:`Triggered`
    (`self.AddControllerYawInput` ActionValue_X)
    (`self.AddControllerPitchInput` ActionValue_Y)))

(event `EnhancedInput|/Game/Integers/IA_Move`
  (params (ActionValue :type "Vector2D Structure") (ElapsedSeconds :type "Float (double-precision)") (TriggeredSeconds :type "Float (double-precision)") (InputAction :type "InputAction Object Reference" :default "/Game/Integers/IA_Move.IA_Move"))
  (bind (_returnvalue_roll _returnvalue_pitch _returnvalue_yaw) (`KismetMathLibrary.BreakRotator` (`self.GetControlRotation`)))
  (bind (_returnvalue_roll_2 _returnvalue_pitch_2 _returnvalue_yaw_2) (`KismetMathLibrary.BreakRotator` (`self.GetControlRotation`)))
  (:`Triggered`
    (`self.AddMovementInput` (`KismetMathLibrary.GetForwardVector` (`KismetMathLibrary.MakeRotator` 0.0 0.0 _returnvalue_yaw_2)) ActionValue_Y)
    (`self.AddMovementInput` (`KismetMathLibrary.GetRightVector` (`KismetMathLibrary.MakeRotator` 0.0 0.0 _returnvalue_yaw)) ActionValue_X)))

(event `EnhancedInput|/Game/Integers/IA_Atack`
  (params (ActionValue :type Boolean) (ElapsedSeconds :type "Float (double-precision)") (TriggeredSeconds :type "Float (double-precision)") (InputAction :type "InputAction Object Reference" :default "/Game/Integers/IA_Atack.IA_Atack"))
  (:`Triggered`
    (`self.Canattack`
      (:`then`
        (set `self.Canattack` false)
        (`|PlayMontage` (`self.Mesh`) (select `int` (`self.Attack_Index`) :`0` "/Game/Animaciones/Punching_Montage.Punching_Montage" :`1` "/Game/Animaciones/Elbow_Punching_Montage.Elbow_Punching_Montage" :`2` "/Game/Animaciones/Kick_Montage.Kick_Montage" :!type "AnimMontage Object Reference")
          (:`then`
            (`/Engine/EditorBlueprintResources/StandardMacros.IncrementInt` (`self.Attack_Index`)))
          (:`OnCompleted`
            (set `self.Canattack` true)
            (set `self.Attack_Index` 0))))
      (:`else`))))

(event `EnhancedInput|/Game/Integers/IA_Run`
  (params (ActionValue :type Boolean) (ElapsedSeconds :type "Float (double-precision)") (TriggeredSeconds :type "Float (double-precision)") (InputAction :type "InputAction Object Reference" :default "/Game/Integers/IA_Run.IA_Run"))
  (bind _charactermovement (`self.CharacterMovement`))
  (:`Triggered`
    (set `CharacterMovementComponent.MaxWalkSpeed` 1500.0 _charactermovement))
  (:`Canceled`
    (set `CharacterMovementComponent.MaxWalkSpeed` 600.0 _charactermovement :!label _label))
  (:`Completed`
    (goto _label)))

(fn `HitDetection`
  (bind _returnvalue (`SceneComponent.GetSocketLocation` (`self.Mesh`) (select `int` (`self.Attack_Index`) :`0` "None" :`1` "LeftHand" :`2` "RightForeArm" :`3` "RightToeBase" :!type "Name")))
  (`KismetSystemLibrary.SphereTraceSingleForObjects` :`Start` _returnvalue :`End` _returnvalue :`Radius` 20.0 :`ObjectTypes` (`|MakeArray` "ObjectTypeQuery1" :!type "EObjectTypeQuery Enum") :`DrawDebugType` "ForOneFrame"))

(fn `UserConstructionScript`)